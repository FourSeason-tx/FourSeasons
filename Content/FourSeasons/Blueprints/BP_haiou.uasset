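; Seagull (haiou) flock actor that flies a configurable number of bird meshes along a looping spline.
; The construction script spawns spline mesh components with random scale, speed, start distance and positional offset, stored in parallel arrays.
; Tick advances each bird by a jittered per-frame step without delta time, orienting it to the spline tangent with a yaw correction.
; A near-equal check against spline length resets its distance to zero.
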(event EventTick
  (params (DeltaSeconds :type Float%20%28single-precision%29))
  (bind _spline (Variables|Default|GetSpline))
  (for (_ _array_index) (Variables|Default|Getniaoooo)
    (Utilities|Array|SetArrayElem (Variables|Default|GetDistanceAlongSpline_shuzu) _array_index (+ (Math|Random|RandomFloatinRange (Utilities|Array|Get(acopy) (Variables|Default|GetSpeed_shuzu) _array_index) (+ (Utilities|Array|Get(acopy) (Variables|Default|GetSpeed_shuzu) _array_index) 0.5)) (Utilities|Array|Get(acopy) (Variables|Default|GetDistanceAlongSpline_shuzu) _array_index)))
    (Transformation|SetRelativeLocationAndRotation (Utilities|Array|Get(acopy) (Variables|Default|Getniaoooo) _array_index) (+ (Spline|GetLocationatDistanceAlongSpline _spline (Utilities|Array|Get(acopy) (Variables|Default|GetDistanceAlongSpline_shuzu) _array_index) "Local") (Utilities|Array|Get(acopy) (Variables|Default|GetNiao_XZ) _array_index)) (Math|Rotator|MakeRotator (.roll (Math|Conversions|RotationFromXVector (Spline|GetDirectionatDistanceAlongSpline _spline (Utilities|Array|Get(acopy) (Variables|Default|GetDistanceAlongSpline_shuzu) _array_index) "Local"))) (.pitch (Math|Conversions|RotationFromXVector (Spline|GetDirectionatDistanceAlongSpline _spline (Utilities|Array|Get(acopy) (Variables|Default|GetDistanceAlongSpline_shuzu) _array_index) "Local"))) (+ (.yaw (Math|Conversions|RotationFromXVector (Spline|GetDirectionatDistanceAlongSpline _spline (Utilities|Array|Get(acopy) (Variables|Default|GetDistanceAlongSpline_shuzu) _array_index) "Local"))) -9e+01)) false false)
    (if (Math|Float|NearlyEqual(Float) (Utilities|Array|Get(acopy) (Variables|Default|GetDistanceAlongSpline_shuzu) _array_index) (Spline|GetSplineLength _spline) (Math|Random|RandomFloatinRange (Utilities|Array|Get(acopy) (Variables|Default|GetSpeed_shuzu) _array_index) (+ (Utilities|Array|Get(acopy) (Variables|Default|GetSpeed_shuzu) _array_index) 0.5)))
      (Utilities|Array|SetArrayElem (Variables|Default|GetDistanceAlongSpline_shuzu) _array_index 0.0))))

(fn ConstructionScript
  (bind _returnvalue (Math|Random|RandomFloatinRange -1.0 1.0))
  (bind _returnvalue_2 (Math|Random|RandomFloatinRange -1.0 1.0))
  (bind _returnvalue_3 (Math|Random|RandomFloatinRange -1.0 1.0))
  (bind _location_x (Variables|Default|GetLocation_X))
  (bind _location_z (Variables|Default|GetLocation_Z))
  (bind _spline (Variables|Default|GetSpline))
  (bind _location_y (Variables|Default|GetLocation_Y))
  (bind _speed (Variables|Default|GetSpeed))
  (bind _returnvalue_4 (* _location_z _returnvalue_2))
  (bind _returnvalue_5 (* _location_x _returnvalue))
  (bind _returnvalue_6 (* _location_y _returnvalue_3))
  (bind _returnvalue_7 (Math|Vector|MakeVector _returnvalue_5 _returnvalue_6 _returnvalue_4))
  (for _index (range 0 (Variables|Default|GetNUM))
    (bind _returnvalue_8 (AddComponent|AddSplineMeshComponent false))
    (Utilities|Array|AddUnique (Variables|Default|GetDistanceAlongSpline_shuzu) (Math|Random|RandomFloatinRange 0.0 6e+03))
    (Utilities|Array|AddUnique (Variables|Default|GetSpeed_shuzu) (Math|Random|RandomFloatinRange _speed (+ _speed 5.0)))
    (Utilities|Array|AddUnique (Variables|Default|Getniaoooo) _returnvalue_8)
    (Utilities|Array|AddUnique (Variables|Default|GetNiao_XZ) _returnvalue_7)
    (Components|StaticMesh|SetStaticMesh _returnvalue_8 (Variables|Default|GetMesh))
    (Rendering|Material|SetMaterial _returnvalue_8 0 (Variables|Default|Getmaterial))
    (Transformation|SetRelativeLocation _returnvalue_8 "0, 0, 0" false false)
    (Transformation|SetRelativeLocation _returnvalue_8 (+ (Spline|GetLocationatDistanceAlongSpline _spline 0.0 "Local") _returnvalue_7) false false)
    (Transformation|SetRelativeRotation _returnvalue_8 (Math|Conversions|RotationFromXVector (Spline|GetDirectionatDistanceAlongSpline _spline 0.0 "Local")) false false)
    (Transformation|AddLocalRotation _returnvalue_8 (Math|Rotator|MakeRotator 0.0 0.0 -9e+01) false false)
    (Transformation|SetRelativeScale3D _returnvalue_8 (Math|Conversions|ToVector(Float) (Math|Random|RandomFloatinRange (Variables|Default|GetScale_MinRND) (Variables|Default|GetScale_MaxRND))))
    (Transformation|AttachComponentToComponent _returnvalue_8 "None" "KeepRelative" "KeepRelative" "KeepRelative" true)))